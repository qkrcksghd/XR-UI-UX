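; Hologram display actor for the fish encyclopedia that shows one entry at a time as an animated model with name, stage and depth text.
; It loads the DT_Encyclopedia row names on BeginPlay, and the Left and Right keys cycle through them with wraparound.
; UpdateHologram checks the player pawn's collected fish, applying M_Hologram to uncollected entries and clearing that material override for collected ones.
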(event Custom|UpdateHologram
  (params (TargetRowName :type Name))
  (bind _hologrammesh (Variables|Default|GetHologramMesh))
  (bind _hologrammesh_2 (Variables|Default|GetHologramMesh))
  (bind _returnvalue (Utilities|GetDataTableRow "/Game/CH/Encyclopedia/DT_Encyclopedia.DT_Encyclopedia" TargetRowName)
    (:then
      (bind _asbp_player_pawn (Utilities|Casting|CastToBP_PlayerPawn (Game|Player|GetPlayerPawn 0)))
      (if (Utilities|Array|ContainsItem (Variables|/Game/CH/BP_PlayerPawn.BP_PlayerPawn_C|GetMyCollectedFish _asbp_player_pawn) TargetRowName)
        (Components|SkeletalMesh|SetSkeletalMeshAsset _hologrammesh (.modelmesh _returnvalue))
        (Rendering|Material|SetMaterial _hologrammesh 0 0)
        (Components|Animation|PlayAnimation _hologrammesh 0 true)
        (Rendering|Components|TextRender|SetText (Variables|Default|GetText_Name) (.name _returnvalue))
        (Rendering|Components|TextRender|SetText (Variables|Default|GetText_Stage) (Utilities|Text|FormatText "{LV} 단계" 0))
        (Rendering|Components|TextRender|SetText (Variables|Default|GetText_Depth) (Utilities|Text|FormatText "수심: {VAL} m" (Utilities|Text|ToText(Float) 0.0 "HalfToEven")))
        (else
          (Components|SkeletalMesh|SetSkeletalMeshAsset _hologrammesh_2 (.modelmesh _returnvalue))
          (Rendering|Material|SetMaterial _hologrammesh_2 0 "/Game/CH/Encyclopedia/M_Hologram.M_Hologram")
          (Components|Animation|PlayAnimation _hologrammesh_2 0 true)
          (Rendering|Components|TextRender|SetText (Variables|Default|GetText_Name) (.name _returnvalue))
          (Rendering|Components|TextRender|SetText (Variables|Default|GetText_Stage) (Utilities|Text|FormatText "{LV} 단계" (.stagelevel _returnvalue)))
          (Rendering|Components|TextRender|SetText (Variables|Default|GetText_Depth) (Utilities|Text|FormatText "수심: {VAL} m" (Utilities|Text|ToText(Float) 0.0 "HalfToEven"))))))))

(event EventBeginPlay
  (bind _outrownames (DataTable|GetDataTableRowNames "/Game/CH/Encyclopedia/DT_Encyclopedia.DT_Encyclopedia"))
  (bind _output_get (Variables|Default|SetRowList _outrownames))
  (CallFunction|UpdateHologram (Utilities|Array|Get(acopy) _output_get)))

(event Input|KeyboardEvents|Right
  (params (Key :type Key%20Structure :default "None"))
  (bind _rowlist (Variables|Default|GetRowList))
  (:Pressed
    (bind _output_get (Variables|Default|SetCurrentIndex (Math|Integer|%(Integer) (+ 1 (Variables|Default|GetCurrentIndex)) (+ (Utilities|Array|LastIndex _rowlist) 1))))
    (CallFunction|UpdateHologram (Utilities|Array|Get(acopy) _rowlist _output_get))))

(event Input|KeyboardEvents|Left
  (params (Key :type Key%20Structure :default "None"))
  (bind _rowlist (Variables|Default|GetRowList))
  (:Pressed
    (if (== (Variables|Default|GetCurrentIndex) 0)
      (bind _output_get (Variables|Default|SetCurrentIndex (Utilities|Array|LastIndex _rowlist)))
      (else
        (Variables|Default|SetCurrentIndex (+ -1 (Variables|Default|GetCurrentIndex)))))
    (CallFunction|UpdateHologram (Utilities|Array|Get(acopy) _rowlist _output_get))))

(fn ConstructionScript)