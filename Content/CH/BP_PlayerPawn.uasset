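; Player pawn for an underwater fish-scanning game that darkens and blue-tints the camera as it descends.
; Tick maps Z to an interpolated post-process color gain.
; While F is held, a headlight sphere trace times focus on one fish, then records its row name and calls OnScanned if new.
; O toggles a hologram display; T spawns a reusable scanner, later teleporting it to the pawn and calling DoScan.
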(event EventTick
  (params (DeltaSeconds :type Float%20%28single-precision%29))
  (bind _returnvalue (Actor|GetComponentbyClass "/Script/Engine.CameraComponent"))
  (bind _headflashlight (Variables|Default|GetHeadFlashlight))
  (bind _returnvalue_2 (Transformation|GetWorldLocation _headflashlight))
  (Utilities|FlowControl|Sequence
    (:then_0
      (Variables|Default|SetTargetGain (Math|Float|MapRangeClamped (.Z (Math|Vector|BreakVector (Transformation|GetActorLocation self))) 0.0 -6e+03 1.0 0.3))
      (Variables|Default|SetCurrentGain (Math|Interpolation|FInterpTo (Variables|Default|GetCurrentGain) (Variables|Default|GetTargetGain) DeltaSeconds (Variables|Default|GetGainInterpSpeed)))
      (bind _structout (Utilities|Struct|SetmembersinPostProcessSettings (Variables|/Script/Engine.CameraComponent|GetPostProcessSettings _returnvalue) (Math|Vector4|MakeVector4 (* 0.7 (Variables|Default|GetCurrentGain)) (* 0.85 (Variables|Default|GetCurrentGain)) (* (Variables|Default|GetCurrentGain) 1.0) 1.0)))
      (Variables|/Script/Engine.CameraComponent|SetPostProcessSettings _returnvalue _structout))
    (:then_1
      (if (Variables|Default|GetIsScanning)
        (bind _outhit (Collision|SphereTraceByChannel _returnvalue_2 (+ _returnvalue_2 (* (Math|Vector|GetForwardVector _headflashlight) "1000.000000,1000.000000,1000.000000")) 1.5e+02 "TraceTypeQuery1" false 0 "None"))
        (bind _asbp_fish_base (Utilities|Casting|CastToBP_FishBase (.HitActor (Collision|BreakHitResult _outhit)))
          (:then
            (if (== (Variables|Default|GetTargetFish) _asbp_fish_base)
              (bind _output_get (Variables|Default|SetScanTime (+ (Utilities|Time|GetWorldDeltaSeconds) (Variables|Default|GetScanTime))))
              (Development|PrintString (Utilities|String|ToString(Float) _output_get))
              (if (>= (Variables|Default|GetScanTime) 3.0)
                (if (not (Utilities|Array|ContainsItem (Variables|Default|GetMyCollectedFish) (Variables|/Game/SY/BP/BP_FishBase.BP_FishBase_C|GetFishRowName _asbp_fish_base)))
                  (Utilities|Array|Add (Variables|Default|GetMyCollectedFish) (Variables|/Game/SY/BP/BP_FishBase.BP_FishBase_C|GetFishRowName _asbp_fish_base))
                  (Development|PrintString (Utilities|String|ToString(Name) (Variables|/Game/SY/BP/BP_FishBase.BP_FishBase_C|GetFishRowName _asbp_fish_base)))
                  (Default|OnScanned _asbp_fish_base)))
              (else
                (Variables|Default|SetTargetFish _asbp_fish_base)
                (Variables|Default|SetScanTime 0.0))))
          (:CastFailed
            (Variables|Default|SetScanTime 0.0)))))))

(event Input|KeyboardEvents|T
  (params (Key :type Key%20Structure :default "None"))
  (:Pressed
    (if (Variables|Default|GetSpawnedScanner?)
      (Transformation|SetActorLocation (Variables|Default|GetScanner) (Transformation|GetActorLocation) false true)
      (Default|DoScan (Variables|Default|GetScanner))
      (else
        (bind _returnvalue (Game|SpawnActorfromClass "/Game/Sonar/BP_Scanner.BP_Scanner_C" (Math|Conversions|ToTransform(Vector) (Transformation|GetActorLocation)) "AlwaysSpawn" "MultiplyWithRoot" 0 0))
        (Variables|Default|SetScanner _returnvalue)
        (Variables|Default|SetSpawnedScanner? true)))))

(event Input|KeyboardEvents|F
  (params (Key :type Key%20Structure :default "None"))
  (:Pressed
    (Variables|Default|SetIsScanning true))
  (:Released
    (Variables|Default|SetIsScanning false)
    (Variables|Default|SetTargetFish 0)))

(event Input|KeyboardEvents|O
  (params (Key :type Key%20Structure :default "None"))
  (:Pressed
    (Utilities|IsValid (Variables|Default|GetHologramRef)
      (:Is%20Valid
        (Actor|DestroyActor (Variables|Default|GetHologramRef)))
      (:Is%20Not%20Valid
        (bind _returnvalue (Game|SpawnActorfromClass "/Game/CH/BP_HologramDisplay.BP_HologramDisplay_C" (Transformation|GetWorldTransform (Variables|Default|GetArrow)) "Undefined" "MultiplyWithRoot" 0 0))
        (Variables|Default|SetHologramRef _returnvalue)))))

(fn ConstructionScript)