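; XR player pawn for an underwater fish-scanning game, handling depth-based view tint and scanner UI.
; Each tick maps world Z to a smoothed post-process gain on the camera, darkening with depth under a blue bias.
; Scan events drive a progress widget through update, reset and delayed hide on completion, and sonar spawn links the sonar to the indicator widget.
; The encyclopedia collected check after a scan has no follow-up logic.
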(event EventOnFishScanned
  (params (Fish :type Actor%20Object%20Reference))
  (Utilities|FlowControl|Sequence
    (:then_0
      (bind _aswbp_scan_progress (Utilities|Casting|CastToWBP_ScanProgress (UserInterface|GetWidget (Variables|Default|GetScanWidget))))
      (Default|ShowComplete _aswbp_scan_progress))
    (:then_1
      (Utilities|FlowControl|Delay 1.5)
      (Development|SetHiddeninGame (Variables|Default|GetScanWidget) true false))
    (:then_2
      (bind _asbp_fish_base (Utilities|Casting|CastToBP_FishBase Fish))
      (if (Class|EncyclopediaSubsystem|IsCollected (Subsystems|GetEncyclopediaSubsystem) (Variables|/Game/SY/BP/BP_FishBase.BP_FishBase_C|GetFishRowName _asbp_fish_base))
        _))))

(event EventOnScanProgress
  (params (Fish :type Actor%20Object%20Reference) (Percent :type Float%20%28single-precision%29))
  (bind _scanwidget (Variables|Default|GetScanWidget))
  (Development|SetHiddeninGame _scanwidget false false)
  (bind _aswbp_scan_progress (Utilities|Casting|CastToWBP_ScanProgress (UserInterface|GetWidget _scanwidget)))
  (Default|SetProgress _aswbp_scan_progress Percent))

(event EventOnSonarSpawned
  (params (Sonar :type Actor%20Object%20Reference))
  (bind _aswbp_indicator (Utilities|Casting|CastToWBP_Indicator (UserInterface|GetUserWidgetObject (Variables|Default|GetIndicatorWidget))))
  (bind _asbp_sonar (Utilities|Casting|CastToBP_Sonar Sonar))
  (Utilities|IsValid Sonar
    (:Is%20Valid
      (Variables|/Game/Arrow/WBP_Indicator.WBP_Indicator_C|SetScannerRef _aswbp_indicator _asbp_sonar))))

(event EventOnScanReset
  (bind _scanwidget (Variables|Default|GetScanWidget))
  (bind _aswbp_scan_progress (Utilities|Casting|CastToWBP_ScanProgress (UserInterface|GetWidget _scanwidget)))
  (Development|SetHiddeninGame _scanwidget true false)
  (Default|ResetUI _aswbp_scan_progress))

(event EventTick
  (params (DeltaSeconds :type Float%20%28single-precision%29))
  (bind _returnvalue (Actor|GetComponentbyClass "/Script/Engine.CameraComponent"))
  (|CallParentFunction DeltaSeconds)
  (Variables|Default|SetTargetGain (Math|Float|MapRangeClamped (.Z (Math|Vector|BreakVector (Transformation|GetActorLocation self))) 0.0 -6e+03 1.0 0.3))
  (Variables|Default|SetCurrentGain (Math|Interpolation|FInterpTo (Variables|Default|GetCurrentGain) (Variables|Default|GetTargetGain) DeltaSeconds (Variables|Default|GetGainInterpSpeed)))
  (bind _structout (Utilities|Struct|SetmembersinPostProcessSettings (Variables|/Script/Engine.CameraComponent|GetPostProcessSettings _returnvalue) (Math|Vector4|MakeVector4 (* 0.7 (Variables|Default|GetCurrentGain)) (* 0.85 (Variables|Default|GetCurrentGain)) (* (Variables|Default|GetCurrentGain) 1.0) 1.0)))
  (Variables|/Script/Engine.CameraComponent|SetPostProcessSettings _returnvalue _structout))

(event EventBeginPlay)

(fn ConstructionScript)