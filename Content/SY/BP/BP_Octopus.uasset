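; BP_Octopus is an actor that wanders on its own with a swimming-like drifting motion.
; Timer-driven events periodically pick a random forward speed and a random yaw offset from its current heading.
; Tick eases toward both targets, moves the actor forward without sweeping for collision, and sets its height to a sine bob around the Z captured at BeginPlay.
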(event Custom|UpdateTargetDirection
  (Variables|Default|SetTargetRotation (Math|Rotator|MakeRotator 0.0 0.0 (+ (.Yaw (Math|Rotator|BreakRotator (Transformation|GetActorRotation))) (Math|Random|RandomFloatinRange -7e+01 7e+01))))
  (Utilities|Time|SetTimerbyEvent (EventDispatchers|CreateEvent :!event Custom|UpdateTargetDirection) (Math|Random|RandomFloatinRange 2.5 4.5)))

(event Custom|UpdateTargetSpeed
  (Variables|Default|SetTargetSpeed (Math|Random|RandomFloatinRange 3.2e+02 4.2e+02))
  (Utilities|Time|SetTimerbyEvent (EventDispatchers|CreateEvent :!event Custom|UpdateTargetSpeed) 2.0))

(event EventBeginPlay
  (Variables|Default|SetBaseZ (.Z (Math|Vector|BreakVector (Transformation|GetActorLocation))))
  (Variables|Default|SetTargetRotation (Transformation|GetActorRotation))
  (CallFunction|UpdateTargetSpeed)
  (CallFunction|UpdateTargetDirection))

(event Collision|EventActorBeginOverlap
  (params (OtherActor :type Actor%20Object%20Reference)))

(event EventTick
  (params (DeltaSeconds :type Float%20%28single-precision%29))
  (bind _returnvalue (Transformation|GetActorLocation))
  (bind (_x _y) (Math|Vector|BreakVector _returnvalue))
  (Variables|Default|SetCurrentSpeed (Math|Interpolation|FInterpTo (Variables|Default|GetCurrentSpeed) (Variables|Default|GetTargetSpeed) DeltaSeconds 1.5))
  (Transformation|SetActorRotation (Math|Interpolation|RInterpTo (Transformation|GetActorRotation) (Variables|Default|GetTargetRotation) DeltaSeconds (Variables|Default|GetTurnInterpSpeed)))
  (Transformation|AddActorWorldOffset (* (Transformation|GetActorForwardVector) (* (Variables|Default|GetCurrentSpeed) DeltaSeconds)))
  (Variables|Default|SetElapsedTime (+ (Variables|Default|GetElapsedTime) DeltaSeconds))
  (Transformation|SetActorLocation (Math|Vector|MakeVector _x _y (+ (* (Math|Trig|Sin(Radians) (* (Variables|Default|GetElapsedTime) (Variables|Default|GetFloatFrequency))) (Variables|Default|GetFloatAmplitude)) (Variables|Default|GetBaseZ))) false false))

(fn ConstructionScript)