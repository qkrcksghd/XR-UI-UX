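; BP_Item is an item actor in the Sonar folder that can be briefly highlighted with an outline visible through objects.
; HighlightItem enables custom depth on the Cube mesh with a stencil value, then turns it off after a two-second delay.
; An unconnected alternative uses the M_HighlightItem overlay material for an outline that does not show through objects.
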(event Custom|HighlightItem
  (bind _cube (Variables|Default|GetCube))
  ;[0.15 0.15 0.15 0.5] 물체 통과되는 아웃라인
  (Development|PrintString "")
  (Rendering|SetRenderCustomDepth _cube true)
  (Rendering|SetCustomDepthStencilValue _cube 3)
  (Utilities|FlowControl|Delay 2.0)
  (Rendering|SetRenderCustomDepth (Variables|Default|GetCube) false))

(event EventBeginPlay)

(event Collision|EventActorBeginOverlap
  (params (OtherActor :type Actor%20Object%20Reference)))

(event EventTick
  (params (DeltaSeconds :type Float%20%28single-precision%29)))

(fn ConstructionScript)