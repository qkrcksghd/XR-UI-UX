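; BP_Sonar is a sonar pulse actor that highlights fish and items and finds the nearest tagged target.
; DoScan runs a timeline that scales the actor outward and drives material opacity, with sphere collision enabled during expansion.
; Overlaps highlight fish and items and record the SonarTarget nearest the player.
; Tick updates that target's distance in meters, and delays clear it; the indicator widget creation is disconnected.
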(event OnComponentBeginOverlap(Sphere)
  (params (OverlappedComponent :type Primitive%20Component%20Object%20Reference) (OtherActor :type Actor%20Object%20Reference) (OtherComp :type Primitive%20Component%20Object%20Reference) (OtherBodyIndex :type Integer) (bFromSweep :type Boolean) (SweepResult :type Hit%20Result%20Structure%20%28by%20ref%29))
  (bind _returnvalue (Transformation|GetActorLocation OtherActor))
  (bind _returnvalue_2 (Game|Player|GetPlayerPawn 0))
  (bind _returnvalue_3 (Transformation|GetActorLocation _returnvalue_2))
  (bind _returnvalue_4 (Math|Vector|Distance(Vector) _returnvalue_3 _returnvalue))
  (Utilities|FlowControl|Sequence
    (:then_0
      (bind _asbp_fish_base (Utilities|Casting|CastToBP_FishBase OtherActor))
      (Development|PrintString "Glow")
      (Default|Highlight _asbp_fish_base))
    (:then_1
      (if (Actor|ActorHasTag OtherActor "SonarTarget")
        (if (< _returnvalue_4 (Variables|Default|GetClosestDistance))
          (Variables|Default|SetClosestDistance _returnvalue_4)
          (Variables|Default|SetClosestActor OtherActor)
          (Development|PrintString (Utilities|String|Append "DIstance: " (Utilities|String|ToString(Float) (Math|Conversions|ToFloat(Integer) (Math|Float|Round (/ _returnvalue_4 1e+02)))) "m"))
          ;[0.15 0.15 0.15 0.5] 10초 후 ClosestActor 초기화
          (Utilities|FlowControl|Delay 2e+01)
          (Variables|Default|SetClosestActor 0)
          (Variables|Default|SetClosestDistance 999999.0))))
    (:then_2
      (bind _asbp_item (Utilities|Casting|CastToBP_Item OtherActor))
      (Default|HighlightItem _asbp_item))))

(event Custom|DoScan
  (Variables|Default|SetClosestDistance 999999.0)
  (Variables|Default|SetClosestActor 0)
  (Rendering|SetActorHiddenInGame false)
  (Collision|SetCollisionEnabled (Variables|Default|GetSphere) "QueryOnly")
  (bind (_direction _scanner_opacity _scannner_expand_size) (Timeline|ExpandScanner PlayFromStart)
    (:Update
      (Transformation|SetActorScale3D (Math|Conversions|ToVector(Float) _scannner_expand_size))
      (Rendering|Material|SetScalarParameterValueonMaterials (Variables|Default|GetSphere) "Scanner_Opacity" _scanner_opacity))
    (:Finished
      (Collision|SetCollisionEnabled (Variables|Default|GetSphere) "NoCollision")
      (Transformation|SetActorScale3D "0, 0, 0")
      (Rendering|SetActorHiddenInGame false))))

(event EventBeginPlay
  (Utilities|Casting|CastToBP_XRPawn (Game|Player|GetPlayerPawn 0)))

(event Collision|EventActorBeginOverlap
  (params (OtherActor :type Actor%20Object%20Reference)))

(event EventTick
  (params (DeltaSeconds :type Float%20%28single-precision%29))
  (if (Utilities|IsValid (Variables|Default|GetClosestActor))
    (Variables|Default|SetClosestDistanceMeters (Math|Float|Round (/ (Math|Vector|Distance(Vector) (Transformation|GetActorLocation (Game|Player|GetPlayerPawn 0)) (Transformation|GetActorLocation (Variables|Default|GetClosestActor))) 1e+02)))
    ;[0.15 0.15 0.15 0.5] 10초 후 ClosestActor 초기화
    (Utilities|FlowControl|Delay 2e+01)
    (Variables|Default|SetClosestActor 0)
    (Variables|Default|SetClosestDistance 999999.0)))

(fn ConstructionScript)